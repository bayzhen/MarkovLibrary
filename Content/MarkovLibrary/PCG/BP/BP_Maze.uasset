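; BP_Maze is an unfinished maze generator Blueprint, apparently intended to use Prim's algorithm.
; It stores cells and walls in a flat MazeMatrix sized on a doubled-plus-one W by H grid, with math expressions mapping X/Y to indices.
; GenerateMazeMatrix only resets the matrix on a length mismatch with W*H.
; BreakWall only builds neighbor positions, PrimMaze and CalculateMazeMatrix are empty, and the construction script calls nothing.
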(event EventBeginPlay)

(event Collision|EventActorBeginOverlap
  (params (OtherActor :type Actor%20Object%20Reference)))

(event EventTick
  (params (DeltaSeconds :type Float%20%28single-precision%29)))

(fn ConstructionScript
  (Utilities|FlowControl|Sequence))

(fn ResetMazeMatrix
  (Utilities|Array|Clear (Variables|Default|GetMazeMatrix))
  (Utilities|Array|Resize (Variables|Default|GetMazeMatrix) (|((({4192924C-4C26-64B3-1F50-AE8625001E9B}*2)+1)*(({E9552EEF-410F-B7D3-1A27-6A82C27D9F76}*2)+1)))))

(fn GenerateMazeMatrix
  (if (!= (Utilities|Array|Length (Variables|Default|GetMazeMatrix)) (* (Variables|Default|GetW) (Variables|Default|GetH)))
    (CallFunction|ResetMazeMatrix)
    (else
      (Development|PrintString "Hello"))))

(fn GetMazePosition
  (params (X :type Integer) (Y :type Integer))
  (return (Utilities|Array|Get(acopy) (Variables|Default|GetMazeMatrix) (|((((2*(X+1))-1)*{E9552EEF-410F-B7D3-1A27-6A82C27D9F76})+((Y+1)*2)) X Y))))

(fn CalculateMazeMatrix)

(fn PrimMaze)

(fn BreakWall
  (params (P :type S%202D%20Position%20Structure))
  (LocalVariables|SetP%20X (.x P))
  (LocalVariables|SetP%20Y (.y P))
  ;[1 1 1] 计算上下左右四个点的位置，移除已经破开的位置和不合理的位置，如果还存在位置，破墙，返回成功，如果不存在，返回失败。
  (LocalVariables|SetUp (Utilities|Struct|MakeS_2DPosition (|(x+1) (LocalVariables|GetP%20X)) (LocalVariables|GetP%20Y)))
  (LocalVariables|SetDown (Utilities|Struct|MakeS_2DPosition (|(x-1) (LocalVariables|GetP%20X)) (LocalVariables|GetP%20Y)))
  (LocalVariables|SetLeft (Utilities|Struct|MakeS_2DPosition (LocalVariables|GetP%20X) (|(y+1) (LocalVariables|GetP%20Y))))
  (LocalVariables|SetDown (Utilities|Struct|MakeS_2DPosition (LocalVariables|GetP%20X) (|(y-1) (LocalVariables|GetP%20Y)))))