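; Cross-platform drag controller that moves pillar instances of a hierarchical instanced static mesh with the mouse or a finger.
; Each tick it traces object types for a ground point, drawn as a debug sphere, and picks an instance by Visibility trace while none is selected.
; The picked index maps through SortActorRef to a main index, which moves to that point.
; Release clears the selection; the pressed flag is never read here.
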(event EventBeginPlay)

(event Collision|EventActorBeginOverlap
  (params (OtherActor :type Actor%20Object%20Reference)))

(event EventTick
  (params (DeltaSeconds :type Float%20%28single-precision%29))
  (bind _returnvalue (Game|GetPlayerController 0))
  (bind _returnvalue_2 (Game|GetPlatformName))
  (bind _returnvalue_3 (Game|GetPlayerController 0))
  (bind _returnvalue_4 (Game|GetPlatformName))
  (bind _returnvalue_5 (Game|GetPlayerController 0))
  (bind _returnvalue_6 (Game|GetPlayerController 0))
  (bind _object_types (Variables|Default|GetObject%20Types))
  (bind _object_types_2 (Variables|Default|GetObject%20Types))
  (bind (_hitresult _returnvalue_7) (Class|PlayerController|GetHitResultUnderCursorforObjects _returnvalue_6 _object_types true))
  (bind (_hitresult_2 _returnvalue_8) (Class|PlayerController|GetHitResultUnderFingerforObjects _returnvalue "Touch1" _object_types_2 true))
  (bind (_hitresult_3 _returnvalue_9) (Game|Player|GetHitResultUnderCursorbyChannel _returnvalue_3 "TraceTypeQuery1" true))
  (bind (_hitresult_4 _returnvalue_10) (Class|PlayerController|GetHitResultUnderFingerbyChannel _returnvalue_5 "Touch1" "TraceTypeQuery1" true))
  (bind _location (Collision|BreakHitResult _hitresult_2))
  (bind _location_2 (Collision|BreakHitResult _hitresult))
  (bind (_bblockinghit _binitialoverlap _time _distance _location_3 _impactpoint _normal _impactnormal _physmat _hitactor _hitcomponent _hitbonename _bonename _hititem) (Collision|BreakHitResult _hitresult_3))
  (bind (_bblockinghit_2 _binitialoverlap_2 _time_2 _distance_2 _location_4 _impactpoint_2 _normal_2 _impactnormal_2 _physmat_2 _hitactor_2 _hitcomponent_2 _hitbonename_2 _bonename_2 _hititem_2) (Collision|BreakHitResult _hitresult_4))
  (Utilities|FlowControl|Sequence
    (:then_0
      (switch string _returnvalue_2
        (:Default
          (Development|PrintString _returnvalue_2))
        (:Windows
          ;[1 1 1] 检查并获取cursor位置，碰撞点在地面。
          (if _returnvalue_7 :!label _label
            (Rendering|Debug|DrawDebugSphere _location_2 1e+02 12 "(R=1.000000,G=0.121763,B=0.000000,A=1.000000)" 0.0)
            (Variables|Default|SetCursorLocation _location_2)))
        (:Mac
          (goto _label))
        (:IOS
          ;[1 1 1] Comment
          (if _returnvalue_8 :!label _label_2
            (Rendering|Debug|DrawDebugSphere _location 1e+02 12 "(R=1.000000,G=0.121763,B=0.000000,A=1.000000)" 0.0)
            (Variables|Default|SetCursorLocation _location)))
        (:Android
          (goto _label_2))))
    (:then_1
      ;[1 1 1] 获取cursor下的HISM ITEM INDEX
      (if (not (Variables|Default|GetSelected))
        (switch string _returnvalue_4
          (:Default
            (Development|PrintString _returnvalue_4))
          (:Windows
            (if _returnvalue_9 :!label _label_3
              (Utilities|Casting|CastToHierarchicalInstancedStaticMeshComponent _hitcomponent)
              (Variables|Default|SetHit%20HISM%20Item _hititem)
              (Variables|Default|SetSelected true)))
          (:Mac
            (goto _label_3))
          (:IOS
            (if _returnvalue_10 :!label _label_4
              (Utilities|Casting|CastToHierarchicalInstancedStaticMeshComponent _hitcomponent_2)
              (Variables|Default|SetHit%20HISM%20Item _hititem_2)
              (Variables|Default|SetSelected true)))
          (:Android
            (goto _label_4)))))
    (:then_2
      ;[1 1 1] 设置柱子的位置
      (if (>= (Variables|Default|GetHit%20HISM%20Item) 0)
        (bind _returnvalue_11 (Class|SortActor|GetMainIndex (Variables|Default|GetSortActorRef) (Variables|Default|GetHit%20HISM%20Item)))
        (Class|SortActor|Move (Variables|Default|GetSortActorRef) _returnvalue_11 (Math|Transform|MakeTransform (Variables|Default|GetCursorLocation)))))))

(event Input|TouchEvents|Touch1
  (params (Key :type Key%20Structure :default "None"))
  (:Pressed
    (Variables|Default|SetbMouseLeftButtonPressed true))
  (:Released
    (Variables|Default|SetbMouseLeftButtonPressed false)
    (Variables|Default|SetSelected false)
    (Variables|Default|SetHit%20HISM%20Item -1)))

(event Input|MouseEvents|LeftMouseButton
  (params (Key :type Key%20Structure :default "None"))
  (:Pressed
    (Variables|Default|SetbMouseLeftButtonPressed true))
  (:Released
    (Variables|Default|SetbMouseLeftButtonPressed false)
    (Variables|Default|SetSelected false)
    (Variables|Default|SetHit%20HISM%20Item -1)))

(fn ConstructionScript)