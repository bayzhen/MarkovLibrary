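; BP_Mazer pairs a BP_Maze child actor with a Cube that Enhanced Input moves in fixed, unswept grid steps.
; The construction script places a downward-facing camera from the maze's width and height.
; A looping timer draws a debug box one step ahead in +X and prints when an overlap test against the Cube's own component hits.
; Alternative line-trace and actor-overlap probes are left unconnected.
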(event Custom|CustomEvent
  (bind _cube (Variables|Default|GetCube))
  (bind _returnvalue (Transformation|GetWorldLocation _cube))
  (bind (_x _y _z) (Class|KismetMathLibrary|BreakVector3f _returnvalue))
  (bind _returnvalue_2 (+ _x 1e+02))
  (bind _returnvalue_3 (Math|Vector|MakeVector _returnvalue_2 _y _z))
  (Rendering|Debug|DrawDebugBox _returnvalue_3 "30.000000,30.000000,60.000000" "(R=1.000000,G=0.000000,B=0.271480,A=1.000000)" "0, 0, 0" 3.0 1e+01)
  (bind _returnvalue_4 (Class|PrimitiveComponent|BoxOverlapComponent (Variables|Default|GetCube) _returnvalue_3 (Variables|Default|GetIn%20Box) true false false))
  (if _returnvalue_4
    (Development|PrintString "Hello")))

(event Input|EnhancedActionEvents|EnhancedInputActionIA_UP
  (params (ActionValue :type Boolean) (ElapsedSeconds :type Float%20%28double-precision%29) (TriggeredSeconds :type Float%20%28double-precision%29) (InputAction :type Input%20Action%20Object%20Reference :default "/Game/MarkovLibrary/Input/IA_UP.IA_UP"))
  (:Started
    (Transformation|AddRelativeLocation (Variables|Default|GetCube) "100.000000,0.000000,0.000000" false false)))

(event Input|EnhancedActionEvents|EnhancedInputActionIA_DOWN
  (params (ActionValue :type Boolean) (ElapsedSeconds :type Float%20%28double-precision%29) (TriggeredSeconds :type Float%20%28double-precision%29) (InputAction :type Input%20Action%20Object%20Reference :default "/Game/MarkovLibrary/Input/IA_DOWN.IA_DOWN"))
  (:Started
    (Transformation|AddRelativeLocation (Variables|Default|GetCube) "-100.000000,0.000000,0.000000" false false)))

(event Input|EnhancedActionEvents|EnhancedInputActionIA_LEFT
  (params (ActionValue :type Boolean) (ElapsedSeconds :type Float%20%28double-precision%29) (TriggeredSeconds :type Float%20%28double-precision%29) (InputAction :type Input%20Action%20Object%20Reference :default "/Game/MarkovLibrary/Input/IA_LEFT.IA_LEFT"))
  (:Started
    (Transformation|AddRelativeLocation (Variables|Default|GetCube) "0.000000,-100.000000,0.000000" false false)))

(event Input|EnhancedActionEvents|EnhancedInputActionIA_RIGHT
  (params (ActionValue :type Boolean) (ElapsedSeconds :type Float%20%28double-precision%29) (TriggeredSeconds :type Float%20%28double-precision%29) (InputAction :type Input%20Action%20Object%20Reference :default "/Game/MarkovLibrary/Input/IA_RIGHT.IA_RIGHT"))
  (:Started
    (Transformation|AddRelativeLocation (Variables|Default|GetCube) "0.000000,100.000000,0.000000" false false)))

(event EventBeginPlay
  (Input|AddMappingContext (PlayerController|LocalPlayerSubsystems|GetEnhancedInputLocalPlayerSubsystem (Game|GetPlayerController 0)) "/Game/MarkovLibrary/Input/IMC.IMC" 0 "(bIgnoreAllPressedKeysUntilRelease=True,bForceImmediately=False)")
  (Utilities|Time|SetTimerbyEvent (delegate Custom|CustomEvent) 0.1 true))

(fn ConstructionScript
  (bind _childactor (Variables|Default|GetChildActor))
  (bind _childactor_2 (Variables|/Script/Engine.ChildActorComponent|GetChildActor _childactor))
  (bind _asbp_maze (Utilities|Casting|CastToBP_Maze _childactor_2))
  (bind _width (Variables|/Script/MarkovLibrary.MyActor|GetWidth _asbp_maze))
  (bind _height (Variables|/Script/MarkovLibrary.MyActor|GetHeight _asbp_maze))
  (Transformation|SetRelativeLocationAndRotation (Variables|Default|GetCamera) (Math|Vector|MakeVector (Math|Conversions|ToFloat(Integer) (* _width 100)) (Math|Conversions|ToFloat(Integer) (* _height 100)) (Math|Conversions|ToFloat(Integer) (* (Math|Integer|Max(Integer) _width _height) 200))) "-90.000000,0.000000,0.000000" false false))