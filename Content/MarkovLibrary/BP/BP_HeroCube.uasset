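; BP_HeroCube is an actor that wanders randomly on a 100-unit grid along the world X and Y axes.
; A fast looping timer started on BeginPlay picks one of the four directions and passes that step to MoveOffset.
; MoveOffset traces vertically down to the target position on the Visibility channel and applies the unswept world offset only when nothing is hit.
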(event Custom|MoveRandom
  (switch int (Math|Random|RandomInteger 4)
    (:0
      (Variables|Default|SetOffset (Math|Vector|MakeVector 1e+02 0.0 0.0)))
    (:1
      (Variables|Default|SetOffset (Math|Vector|MakeVector -1e+02 0.0 0.0)))
    (:2
      (Variables|Default|SetOffset (Math|Vector|MakeVector 0.0 1e+02 0.0)))
    (:3
      (Variables|Default|SetOffset (Math|Vector|MakeVector 0.0 -1e+02 0.0))))
  (CallFunction|MoveOffset (Variables|Default|GetOffset)))

(event EventBeginPlay
  (Utilities|Time|SetTimerbyEvent (delegate Custom|MoveRandom) 0.03 true))

(fn ConstructionScript)

(fn MoveOffset
  (params (Offset :type Vector))
  (LocalVariables|SetA1 Offset)
  (bind _returnvalue (Collision|LineTraceByChannel (+ (+ (LocalVariables|GetA1) (Transformation|GetActorLocation)) "0.000000,0.000000,200.000000") (+ (LocalVariables|GetA1) (Transformation|GetActorLocation)) "TraceTypeQuery1" false 0 "None"))
  (if (not _returnvalue)
    (Transformation|AddActorWorldOffset (LocalVariables|GetA1))))