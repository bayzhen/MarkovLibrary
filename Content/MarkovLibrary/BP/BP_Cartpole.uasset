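; BP_Cartpole is a cart-pole environment that exposes movement actions and observations.
; ActionA and ActionD slide the Cube cart along local X, scaled by frame time, and are also triggered by Enhanced Input keys.
; BeginPlay adds the input mapping and randomly offsets the cart's start position.
; GetObs returns cart X, Cube1 pitch and a Truncated flag, which is set when the physics constraint breaks.
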(event OnConstraintBroken(PhysicsConstraint)
  (params (ConstraintIndex :type Integer))
  (Variables|Default|SetTruncated true)
  (Development|PrintString "Hello"))

(event Custom|Action%20A
  (Transformation|AddLocalOffset (Variables|Default|GetCube) (Math|Vector|MakeVector (* (Utilities|Time|GetWorldDeltaSeconds) (Variables|Default|GetBaseMoveSpeed) -1.0) 0.0 0.0) false false))

(event Custom|Action%20D
  (Transformation|AddLocalOffset (Variables|Default|GetCube) (Math|Vector|MakeVector (* (Utilities|Time|GetWorldDeltaSeconds) (Variables|Default|GetBaseMoveSpeed)) 0.0 0.0) false false))

(event Input|EnhancedActionEvents|EnhancedInputActionIA_A
  (params (ActionValue :type Boolean) (ElapsedSeconds :type Float%20%28double-precision%29) (TriggeredSeconds :type Float%20%28double-precision%29) (InputAction :type Input%20Action%20Object%20Reference :default "/Game/MarkovLibrary/Input/IA_A.IA_A"))
  (:Triggered
    (Transformation|AddLocalOffset (Variables|Default|GetCube) (Math|Vector|MakeVector (* (Utilities|Time|GetWorldDeltaSeconds) (Variables|Default|GetBaseMoveSpeed) -1.0) 0.0 0.0) false false)))

(event Input|EnhancedActionEvents|EnhancedInputActionIA_D
  (params (ActionValue :type Boolean) (ElapsedSeconds :type Float%20%28double-precision%29) (TriggeredSeconds :type Float%20%28double-precision%29) (InputAction :type Input%20Action%20Object%20Reference :default "/Game/MarkovLibrary/Input/IA_D.IA_D"))
  (:Triggered
    (Transformation|AddLocalOffset (Variables|Default|GetCube) (Math|Vector|MakeVector (* (Utilities|Time|GetWorldDeltaSeconds) (Variables|Default|GetBaseMoveSpeed)) 0.0 0.0) false false)))

(event EventBeginPlay
  (Input|AddMappingContext (PlayerController|LocalPlayerSubsystems|GetEnhancedInputLocalPlayerSubsystem (Game|GetPlayerController 0)) "/Game/MarkovLibrary/Input/IMC.IMC" 0 "(bIgnoreAllPressedKeysUntilRelease=True,bForceImmediately=False)")
  (Transformation|AddLocalOffset (Variables|Default|GetCube) (Math|Vector|MakeVector (* (- (Math|Random|RandomFloat) 0.5) 1e+02) 0.0 0.0) false false))

(fn ConstructionScript)

(fn GetObs
  (return (.x (Transformation|GetWorldLocation (Variables|Default|GetCube))) (.pitch (Transformation|GetWorldRotation (Variables|Default|GetCube1))) (Variables|Default|GetTruncated)))